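; Player character for a 2D side-scrolling game, with sprint, jump, health and a time-based score.
; Input drives movement, pause and stamina-limited sprinting and jumping, while enemy-tagged overlaps subtract that enemy's damage from health.
; Tick swaps idle and running flipbooks, flips facing through control rotation, then updates stamina and the HUD.
; Zero health pauses the game, replaces all widgets with a death screen showing the final score.
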(event `self.ReceiveBeginPlay`
  ;[1 1 1] Handle Construction
  (`ActorComponent.SetIsReplicated` (`self.Sprite`) true)
  (`self.Init Interface`)
  (`self.Init Stats`)
  (`WidgetBlueprintLibrary.SetInputMode_GameOnly` (`GameplayStatics.GetPlayerController` 0))
  (bind _returnvalue (`AddComponent|NODE_AddAudioComponent-3`))
  (set `self.Audio Component` _returnvalue))

(event `InputAction|Pause`
  (params (Key :type "Key Structure"))
  (bind _pause (`self.Pause`))
  ;[1 1 1] Pause
  (:`Pressed`
    (`/Engine/EditorBlueprintResources/StandardMacros.IsValid` (`self.Pause`)
      (:`Is Valid`
        _)
      (:`Is Not Valid`
        (bind _returnvalue (`|CreateWidget` "/Game/Blueprints/Player/Pause.Pause_C"))
        (set `self.Pause` _returnvalue)))
    (`WidgetBlueprintLibrary.SetInputMode_UIOnlyEx` (`GameplayStatics.GetPlayerController` 0) _pause)
    (`UserWidget.AddToViewport` _pause 0)
    (`GameplayStatics.SetGamePaused` true)
    (set `PlayerController.bShowMouseCursor` true (`GameplayStatics.GetPlayerController` 0))))

(event `UpdateAnimation`
  ;[1 1 1] Handle Animation
  (`PaperFlipbookComponent.SetFlipbook` (`self.Sprite`) (select `bool` (> (`KismetMathLibrary.VSize` (`self.GetVelocity`)) 0.0) :`false` "/Game/2DSideScroller/Sprites/IdleAnimation.IdleAnimation" :`true` "/Game/2DSideScroller/Sprites/RunningAnimation.RunningAnimation" :!type "PaperFlipbook Object Reference")))

(event `InputAxis|MoveRight`
  (params (AxisValue :type "Float (single-precision)"))
  ;[1 1 1] Handle movement
  (if (> AxisValue 0.0)
    (set `self.bisMovingRight` true)
    (elif (< AxisValue 0.0)
      (set `self.bisMovingRight` false)))
  (`self.AddMovementInput` (1.0 0.0 0.0) AxisValue))

(event `self.ReceiveTick`
  (params (DeltaSeconds :type "Float (single-precision)"))
  ;[1 1 1] Tick - Updates animation
  (`self.UpdateAnimation`)
  (`/Engine/EditorBlueprintResources/StandardMacros.CompareFloat` (.x (`MovementComponent.Velocity` (`self.GetMovementComponent`)))
    (:`>`
      (`Controller.SetControlRotation` (`self.GetController`) (`KismetMathLibrary.MakeRotator` 0.0) :!label _label))
    (:`==`
      (if (`self.bisMovingRight`)
        (goto _label)
        (else
          (`Controller.SetControlRotation` (`self.GetController`) (`KismetMathLibrary.MakeRotator` 0.0 0.0 180.0) :!label _label_2))))
    (:`<`
      (goto _label_2)))
  ;[1 1 1] Tick - Update UI and Death
  (bind _lost (`self.Check Loss`))
  (if _lost
    (`self.Handle Death`)
    (else
      (`self.Handle Interface`))))

(event `self.Damage.OnComponentBeginOverlap`
  (params (OverlappedComponent :type "PrimitiveComponent Object Reference") (OtherActor :type "Actor Object Reference") (OtherComp :type "PrimitiveComponent Object Reference") (OtherBodyIndex :type Integer) (bFromSweep :type Boolean) (SweepResult :type "HitResult Structure (by ref)"))
  ;[1 1 1] Get Hit by Enemy
  (if (and (`self.ActorHasTag` OtherActor "Enemy") (<= 0.0 0.0))
    (bind _asenemy_character (cast `/Game/Blueprints/Enemy/Enemy_Character` OtherActor)
      (:`then`
        (set `self.Health` (- (`self.Health`) (`/Game/Blueprints/Enemy/Enemy_Character.Damage` _asenemy_character)))
        (`AddComponent|NODE_AddAudioComponent-2`))
      (:`CastFailed`
        (`KismetSystemLibrary.PrintString` "Error in Enemy Damage, wrong tag?" true true (struct :`G` 0.66 :`B` 1.0 :`A` 1.0) 4.0)))))

(event `InputAction|Sprint`
  (params (Key :type "Key Structure"))
  ;[1 1 1] Sprint
  (:`Pressed`
    (if (`self.CanJump`)
      (if (> (`self.Stamina`) (`self.Minimum Stamina`))
        (set `self.Sprint` true))
      (else
        (set `self.Sprint` false :!label _label_3)
        (set `CharacterMovementComponent.MaxWalkSpeed` (`self.Walk Speed`) (`self.CharacterMovement`)))))
  (:`Released`
    (goto _label_3)))

(event `InputAction|Jump`
  (params (Key :type "Key Structure"))
  (bind _stamina (`self.Stamina`))
  (bind _jump_exhaust (`self.Jump Exhaust`))
  ;[1 1 1] Handle Jump
  (:`Pressed`
    (if (and (`self.CanJump`) (> _stamina _jump_exhaust)) :!label _label_4
      (set `self.Stamina` (- _stamina _jump_exhaust))
      (`self.Jump`)
      (`AddComponent|NODE_AddAudioComponent-0`)
      (else
        (`self.StopJumping` :!label _label_5))))
  (:`Released`
    (goto _label_5)))

(event `InputTouch`
  (params (Location :type "Vector Structure") (FingerIndex :type "ETouchIndex Enum"))
  ;[1 1 1] Handle Jump
  (:`Pressed`
    (goto _label_4))
  (:`Released`
    (goto _label_5)))

(fn `Check Loss`
  (returns (Lost :type Boolean))
  (if (<= (`self.Health`) 0.0)
    (return true)
    (else
      (return false))))

(fn `Handle Death`
  (bind _returnvalue (`GameplayStatics.GetPlayerController` 0))
  (`GameplayStatics.SetGamePaused` true)
  (`self.Update Health`)
  (`AddComponent|NODE_AddAudioComponent-5`)
  (`WidgetLayoutLibrary.RemoveAllWidgets`)
  (bind _returnvalue_2 (`|CreateWidget` "/Game/Blueprints/Player/Death.Death_C"))
  (set `/Game/Blueprints/Player/Death.Final Score` (`KismetTextLibrary.Conv_DoubleToText` (`self.Player Score`) "HalfToEven") _returnvalue_2)
  (`UserWidget.AddToViewport` _returnvalue_2 0)
  (`WidgetBlueprintLibrary.SetInputMode_UIOnlyEx` _returnvalue _returnvalue_2)
  (set `PlayerController.bShowMouseCursor` true _returnvalue))

(fn `Handle Interface`
  (`self.Update Speed`)
  (`self.Update Health`)
  (`self.Handle Sprint`)
  (`self.Update Stamina`)
  (`self.Update Score`))

(fn `Handle Sprint`
  (if (`self.Sprint`)
    (if (> (`self.Stamina`) 0.0)
      (if (`self.CanJump`)
        (set `self.Stamina` (- (`self.Stamina`) (`self.Sprint Exhaust Rate`)))
        (set `CharacterMovementComponent.MaxWalkSpeed` (`self.Sprint Speed`) (`self.CharacterMovement`)))
      (else
        (set `self.Sprint` false)
        (set `self.Stamina` 0.0)
        (set `CharacterMovementComponent.MaxWalkSpeed` (`self.Walk Speed`) (`self.CharacterMovement`))))
    (elif (< (`self.Stamina`) (`self.Max Stamina`))
      (if (`self.CanJump`)
        (set `self.Stamina` (+ (`self.Stamina`) (`self.Sprint Recovery Rate`))))
      (else
        (set `self.Stamina` (`self.Max Stamina`))))))

(fn `Init Interface`
  (bind _returnvalue (`|CreateWidget` "/Game/Blueprints/Player/Player_UI.Player_UI_C"))
  (bind _output_get (set `self.UI` _returnvalue))
  (`UserWidget.AddToViewport` _output_get 0)
  (bind _returnvalue_2 (`|CreateWidget` "/Game/Blueprints/Player/Pause.Pause_C"))
  (set `self.Pause` _returnvalue_2))

(fn `Init Stats`
  (set `self.Stamina` (`self.Max Stamina`))
  (set `self.Health` (`self.Max Health`))
  (set `self.Player Score` 0.0))

(fn `Update Health`
  (`ProgressBar.SetPercent` (`/Game/Blueprints/Player/Player_UI.Health` (`self.UI`)) (/ (`self.Health`) (`self.Max Health`))))

(fn `Update Score`
  (set `self.Player Score` (`GameplayStatics.GetTimeSeconds`))
  (`EditableText.SetText` (`/Game/Blueprints/Player/Player_UI.CurrentScore` (`self.UI`)) (`KismetTextLibrary.Conv_DoubleToText` (`self.Player Score`) "HalfToEven")))

(fn `Update Speed`
  (`EditableText.SetText` (`/Game/Blueprints/Player/Player_UI.CurrentSpeed` (`self.UI`)) (`KismetTextLibrary.Conv_DoubleToText` (.x (`CharacterMovementComponent.GetLastUpdateVelocity` (`self.CharacterMovement`))) "HalfToEven")))

(fn `Update Stamina`
  (`ProgressBar.SetPercent` (`/Game/Blueprints/Player/Player_UI.Stamina` (`self.UI`)) (/ (`self.Stamina`) (`self.Max Stamina`))))

(fn `UserConstructionScript`)