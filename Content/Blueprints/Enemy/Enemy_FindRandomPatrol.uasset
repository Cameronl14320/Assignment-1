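; Behavior tree task that picks a random patrol destination for an Enemy_Character.
; It sets the character's walk speed to its patrol speed, then writes a random reachable point within PatrolRadius to the PatrolLocation blackboard key.
; If no point is found it writes the pawn's current location instead.
; The task succeeds in both cases and fails only when the pawn is not an Enemy_Character.
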(event `self.ReceiveExecuteAI`
  (params (OwnerController :type "AIController Object Reference") (ControlledPawn :type "Pawn Object Reference"))
  (bind _returnvalue (`Actor.K2_GetActorLocation` ControlledPawn))
  (bind (_randomlocation _returnvalue_2) (`NavigationSystemV1.K2_GetRandomReachablePointInRadius` _returnvalue (`self.Patrol Radius`) null null))
  (bind _asenemy_character (cast `/Game/Blueprints/Enemy/Enemy_Character` ControlledPawn)
    (:`then`
      (`/Game/Blueprints/Enemy/Enemy_Character.Update Walk Speed` _asenemy_character (`/Game/Blueprints/Enemy/Enemy_Character.Patrol Speed` _asenemy_character))
      (if _returnvalue_2
        (`BTFunctionLibrary.SetBlackboardValueAsVector` (`self.Patrol Location`) _randomlocation)
        (else
          (`BTFunctionLibrary.SetBlackboardValueAsVector` (`self.Patrol Location`) _returnvalue)))
      (`self.FinishExecute` true))
    (:`CastFailed`
      (`self.FinishExecute` false))))