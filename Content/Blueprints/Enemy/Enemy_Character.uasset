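; Enemy character for a side-view game that animates a flipbook sprite and turns to face its horizontal movement.
; Each tick it swaps between running and idle flipbooks by speed, then sets controller yaw forward or reversed from the sign of X velocity.
; When X velocity is zero, the BisMovingRight flag decides the facing.
; A separate function sets the character's max walk speed.
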(event `UpdateAnimation`
  ;[1 1 1] Handle Animation
  (`PaperFlipbookComponent.SetFlipbook` (`self.Sprite`) (select `bool` (> (`KismetMathLibrary.VSize` (`self.GetVelocity`)) 10.0) :`false` "/Game/2DSideScroller/Sprites/IdleAnimation.IdleAnimation" :`true` "/Game/2DSideScroller/Sprites/RunningAnimation.RunningAnimation" :!type "PaperFlipbook Object Reference")))

(event `self.ReceiveTick`
  (params (DeltaSeconds :type "Float (single-precision)"))
  ;[1 1 1] Tick - Updates animation
  (`self.UpdateAnimation`)
  (`/Engine/EditorBlueprintResources/StandardMacros.CompareFloat` (.x (`MovementComponent.Velocity` (`self.CharacterMovement`)))
    (:`>`
      (`Controller.SetControlRotation` (`self.GetController`) (`KismetMathLibrary.MakeRotator` 0.0) :!label _label))
    (:`==`
      (if (`self.bisMovingRight`)
        (goto _label)
        (else
          (`Controller.SetControlRotation` (`self.GetController`) (`KismetMathLibrary.MakeRotator` 0.0 0.0 180.0) :!label _label_2))))
    (:`<`
      (goto _label_2))))

(fn `Update Walk Speed`
  (params (`New Walk Speed` :type "Float (double-precision)"))
  (set `CharacterMovementComponent.MaxWalkSpeed` `New Walk Speed` (`self.CharacterMovement`)))

(fn `UserConstructionScript`)