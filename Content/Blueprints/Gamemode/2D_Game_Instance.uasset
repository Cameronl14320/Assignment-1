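; Game instance for the 2D game mode that owns the audio volume settings.
; On Init it waits briefly, activates the global sound mix, then applies the stored master, music and effects volumes.
; SetVolume clamps a value to 0–1, overrides the matching sound class in that mix and writes it back into the SoundOptions struct.
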(event `self.ReceiveInit`
  (bind (_mastervolume _musicvolume _effectsvolume) (break `/Game/Sounds/Settings/Sound_Options` (`self.Sound Options`)))
  (`KismetSystemLibrary.Delay` 0.2)
  (`GameplayStatics.SetBaseSoundMix` "/Game/Sounds/Settings/Mix_Global.Mix_Global")
  (`GameplayStatics.PushSoundMixModifier` "/Game/Sounds/Settings/Mix_Global.Mix_Global")
  (`|ExecutionSequence`
    (:`then_0`
      (`self.SetVolume` "NewEnumerator0" _mastervolume))
    (:`then_1`
      (`self.SetVolume` "NewEnumerator1" _musicvolume))
    (:`then_2`
      (`self.SetVolume` "NewEnumerator2" _effectsvolume))))

(fn `SetVolume`
  (params (`Sound Channels` :type "/Game/Sounds/Settings/Sound_Channels Enum" :default "NewEnumerator0") (Value :type "Float (double-precision)"))
  (bind _returnvalue (`KismetMathLibrary.FClamp` Value))
  (bind _sound_options (`self.Sound Options`))
  (switch `/Game/Sounds/Settings/Sound_Channels` `Sound Channels`
    (:`NewEnumerator0`
      (`GameplayStatics.SetSoundMixClassOverride` "/Game/Sounds/Settings/Mix_Global.Mix_Global" "/Game/Sounds/Settings/Master.Master" _returnvalue)
      (setmembers `/Game/Sounds/Settings/Sound_Options` :`StructRef` _sound_options :`MasterVolume` _returnvalue))
    (:`NewEnumerator1`
      (`GameplayStatics.SetSoundMixClassOverride` "/Game/Sounds/Settings/Mix_Global.Mix_Global" "/Game/Sounds/Settings/Music.Music" _returnvalue)
      (setmembers `/Game/Sounds/Settings/Sound_Options` :`StructRef` _sound_options :`MusicVolume` _returnvalue))
    (:`NewEnumerator2`
      (`GameplayStatics.SetSoundMixClassOverride` "/Game/Sounds/Settings/Mix_Global.Mix_Global" "/Game/Sounds/Settings/Effects.Effects" _returnvalue)
      (setmembers `/Game/Sounds/Settings/Sound_Options` :`StructRef` _sound_options :`EffectsVolume` _returnvalue))))